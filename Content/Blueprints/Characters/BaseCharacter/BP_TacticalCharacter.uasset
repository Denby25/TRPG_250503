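; Base tactical character that tracks health, consciousness and per-character attributes.
; On BeginPlay it creates an owner-linked health bar in its widget component, marks itself conscious and copies turn speed from its attributes as a placeholder.
; AttemptAttack subtracts fixed damage from its own health, and OnDeath ragdolls the mesh and clears consciousness.
; GetFloatAttribute maps an attribute selector to the matching value in MyAttributes.
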(event `self.ReceiveBeginPlay`
  (`|ExecutionSequence`
    (:`then_0`
      (bind _returnvalue (`|CreateWidget` "/Game/Blueprints/Characters/W_HealthBar.W_HealthBar_C"))
      (set `/Game/Blueprints/Characters/W_HealthBar.OwningCharacter` self _returnvalue)
      (`WidgetComponent.SetWidget` (`self.Widget`) _returnvalue)
      (set `self.bIsConscious` true))
    (:`then_1`
      ; Placeholder for proper speed attribute handling
      (set `self.ModifiedTurnSpeed` (`.TurnSpeed_10_396F28A9452AC3767ABD899442F406B8` (break `/Game/Blueprints/Characters/BaseCharacter/CharacterAttributes` (`self.MyAttributes`)))))))

(event `/Game/Blueprints/Characters/BPI_Combat.AttemptAttack`
  (params (DamageData :type "/Game/Blueprints/Core/DamageData Structure") (AttackerData :type "/Game/Blueprints/Characters/BaseCharacter/CharacterAttributes Structure"))
  (bind _output_get (set `self.HealthPoints` (- (`self.HealthPoints`) 30.0)))
  (if (<= _output_get 0.0)
    (`self.OnDeath`)))

(event `OnDeath`
  (bind _mesh (`self.Mesh`))
  (`PrimitiveComponent.SetSimulatePhysics` _mesh true)
  (`PrimitiveComponent.SetCollisionEnabled` _mesh "QueryAndPhysics")
  (set `self.bIsConscious` false))

(fn `GetFloatAttribute`
  (params (Attribute :type "/Game/Blueprints/Characters/BaseCharacter/ECharacterAttributes Enum" :default "NewEnumerator6"))
  (returns (AttributeValue :type "Float (double-precision)"))
  (bind (_level _maxhealth _turnspeed _movementbudget _trackingrecall) (break `/Game/Blueprints/Characters/BaseCharacter/CharacterAttributes` (`self.MyAttributes`)))
  (return (select `/Game/Blueprints/Characters/BaseCharacter/ECharacterAttributes` Attribute :`NewEnumerator0` _maxhealth :`NewEnumerator2` _turnspeed :`NewEnumerator3` _movementbudget :`NewEnumerator5` _trackingrecall)))

(fn `UserConstructionScript`)