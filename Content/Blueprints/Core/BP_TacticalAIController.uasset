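; AI controller for a tactical character that carries out move, jump and attack requests and tracks the characters it perceives.
; Moves walk a path point by point through chained AIMoveTo calls, then signal completion; jumps launch along a suggested projectile arc.
; Attacks face the target and send it damage data when the punch montage completes.
; Perception updates maintain a map of each character's last known location, visibility and allegiance-based enemy status.
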(event `self.ReceiveBeginPlay`
  (bind _asbp_tactical_character (cast `/Game/Blueprints/Characters/BaseCharacter/BP_TacticalCharacter` (`self.K2_GetPawn`)))
  (set `self.ControlledCharacter` _asbp_tactical_character)
  (bind _returnvalue (`GameplayStatics.GetActorOfClass` "/Game/Blueprints/Core/BP_TacticalPlayerController.BP_TacticalPlayerController_C"))
  (set `self.PlayerController` _returnvalue))

(event `/Game/Blueprints/Core/BPI_AIControllerInstructions.RequestMove`
  (params (MovePath :type "Array of Vector Structure (by ref)"))
  (set `self.MovePath` MovePath)
  (set `self.PointCounter` 0)
  (`self.FollowPath`))

(event `FollowPath`
  (bind _movepath (`self.MovePath`))
  (set `self.PathPoints` (`KismetArrayLibrary.Array_Length` _movepath))
  (`|AIMoveTo` (`self.ControlledCharacter`) (`|GetArrayItem` _movepath (`self.PointCounter`)) null 50.0
    (:`OnSuccess`
      (bind _result (`/Engine/EditorBlueprintResources/StandardMacros.IncrementInt` (`self.PointCounter`))
        (:`  `
          (bind _output_get (set `self.PointCounter` _result))
          (if (>= _output_get (`self.PathPoints`))
            (`self.OnFollowPathCompleted`)
            (else
              (`self.FollowPath`))))))))

(event `/Game/Blueprints/Core/BPI_AIControllerInstructions.RequestJump`
  (params (Destination :type "Vector Structure"))
  (bind _outlaunchvelocity (`GameplayStatics.SuggestProjectileVelocity_CustomArc` (`self.K2_GetActorLocation` (`self.ControlledCharacter`)) (`KismetMathLibrary.MakeVector` (.x Destination) (.y Destination) (+ (.z Destination) (`self.JumpAdjustmentZ`))) 0.0 0.4))
  (`Character.LaunchCharacter` (`self.ControlledCharacter`) _outlaunchvelocity true true))

(event `/Game/Blueprints/Core/BPI_AIControllerInstructions.RequestAttack`
  (params (TargetCharacter :type "/Game/Blueprints/Characters/BaseCharacter/BP_TacticalCharacter Object Reference"))
  (bind _controlledcharacter (`self.ControlledCharacter`))
  (`self.K2_SetActorRotation` (`self.ControlledCharacter`) (`KismetMathLibrary.FindLookAtRotation` (`self.K2_GetActorLocation` (`self.ControlledCharacter`)) (`self.K2_GetActorLocation` TargetCharacter)) false)
  (set `self.ActionTarget` TargetCharacter)
  (`|PlayMontage` (`Character.Mesh` (`self.ControlledCharacter`)) "/Game/Characters/Mannequins/Animations/Manny/AM_Punch.AM_Punch"
    (:`OnCompleted`
      (message `/Game/Blueprints/Characters/BPI_Combat.AttemptAttack` TargetCharacter (make `/Game/Blueprints/Core/DamageData` _controlledcharacter) (`/Game/Blueprints/Characters/BaseCharacter/BP_TacticalCharacter.MyAttributes` _controlledcharacter)))))

(event `self.AIPerception.OnTargetPerceptionUpdated`
  (params (Actor :type "Actor Object Reference") (Stimulus :type "AIStimulus Structure"))
  (bind (_age _expirationage _strength _stimuluslocation _receiverlocation _tag _bsuccessfullysensed) (break `AIStimulus` Stimulus))
  (bind _asbp_tactical_character (cast `/Game/Blueprints/Characters/BaseCharacter/BP_TacticalCharacter` Actor))
  (if _bsuccessfullysensed
    (`BlueprintMapLibrary.Map_Add` (`self.PerceivedCharacters`) _asbp_tactical_character (make `/Game/Blueprints/AI/PerceivedCharacterData` _stimuluslocation 0.0 (`self.IsMyEnemy` _asbp_tactical_character) true))
    (else
      (bind _structout (setmembers `/Game/Blueprints/AI/PerceivedCharacterData` :`StructRef` (`BlueprintMapLibrary.Map_Find` (`self.PerceivedCharacters`) _asbp_tactical_character) :`LastKnownLocation` _stimuluslocation :`bIsVisible` false))
      (`BlueprintMapLibrary.Map_Add` (`self.PerceivedCharacters`) _asbp_tactical_character _structout))))

(fn `IsMyEnemy`
  (params (PerceivedCharacter :type "/Game/Blueprints/Characters/BaseCharacter/BP_TacticalCharacter Object Reference"))
  (returns (bIsMyEnemy :type Boolean))
  (bind _allegiance (`/Game/Blueprints/Characters/BaseCharacter/BP_TacticalCharacter.Allegiance` PerceivedCharacter))
  (return (`KismetMathLibrary.BooleanNOR` (== _allegiance (struct :`TagName` "Allegiance.Neutral")) (== _allegiance (`/Game/Blueprints/Characters/BaseCharacter/BP_TacticalCharacter.Allegiance` (`self.ControlledCharacter`))))))

(fn `UserConstructionScript`)