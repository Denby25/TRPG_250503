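; BP_TacticalChar is a tactical character that moves to commanded locations within a limited movement budget.
; ReceiveMovementCommand checks straight-line distance against RemainingMovement, issues SimpleMoveToLocation through its controller and deducts that distance upfront, or prints why the move is refused.
; OnMoveCompleted is an empty hook called immediately after the move is issued, without waiting for arrival.
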(fn `OnMoveCompleted`)

(fn `ReceiveMovementCommand`
  (params (TargetLocation :type "Vector Structure"))
  (locals (localDistance :type "Float (double-precision)" :default 0.0))
  (bind _returnvalue (`KismetMathLibrary.VSize` (- TargetLocation (`self.K2_GetActorLocation`))))
  (if (> (`self.RemainingMovement`) 0.0)
    (set `local.localDistance` _returnvalue)
    (if (<= _returnvalue (`self.RemainingMovement`))
      (`AIBlueprintHelperLibrary.SimpleMoveToLocation` (`self.GetController`) (`local.TargetLocation`))
      (set `self.RemainingMovement` (- (`self.RemainingMovement`) (`local.localDistance`)))
      (`self.OnMoveCompleted`)
      (else
        (`KismetSystemLibrary.PrintString` "Insufficient MP")))
    (else
      (`KismetSystemLibrary.PrintString` "No MP remaining"))))

(fn `UserConstructionScript`)