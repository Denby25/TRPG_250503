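; Player controller for turn-based tactical play, running turn order, action menu, camera and pause state.
; CalculateTurn accumulates randomised Speed-based points until a character reaches the threshold, then has the shared AI controller possess it.
; Choosing Move enables click-to-move through that AI controller.
; The camera pawn follows the active character until manually panned; the spectator-toggle input currently advances turns, leaving its state switch unwired.
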(event `self.ReceiveBeginPlay`
  (bind _returnvalue (subsystem `EnhancedInputLocalPlayerSubsystem`))
  (`|ExecutionSequence`
    (:`then_0`
      (set `self.bShowMouseCursor` true)
      (`/Engine/EditorBlueprintResources/StandardMacros.IsValid` _returnvalue
        (:`Is Valid`
          (`EnhancedInputSubsystemInterface.AddMappingContext` _returnvalue "/Game/Input/IMC_Combat.IMC_Combat" 0 (struct))
          (`EnhancedInputSubsystemInterface.AddMappingContext` _returnvalue "/Game/Input/IMC_Camera.IMC_Camera" 0 (struct)))))
    (:`then_1`
      (bind _returnvalue_2 (`GameplayStatics.GetActorOfClass` "/Game/Blueprints/Core/BP_CameraPawn.BP_CameraPawn_C"))
      (set `self.CameraPawn` _returnvalue_2))
    (:`then_2`
      (bind _returnvalue_3 (`|CreateWidget` "/Game/Blueprints/Menu/WBP_PauseMenu.WBP_PauseMenu_C"))
      (set `self.PauseMenuInstance` _returnvalue_3)
      (bind _returnvalue_4 (`|CreateWidget` "/Game/Blueprints/Menu/WBP_ActionMenu.WBP_ActionMenu_C"))
      (bind _output_get (set `self.ActionMenuInstance` _returnvalue_4))
      (add `/Game/Blueprints/Menu/WBP_ActionMenu.OnActionSelected` _output_get (`|CreateDelegate` :!event `OnActionSelected`))
      (bind _returnvalue_5 (`GameplayStatics.GetActorOfClass` "/Game/Blueprints/Core/BP_TacticalAIController.BP_TacticalAIController_C"))
      (set `self.AIController` _returnvalue_5))
    (:`then_3`
      (set `self.CurrentState` "NewEnumerator0"))
    (:`then_4`
      (bind _outactors (`GameplayStatics.GetAllActorsOfClass` "/Game/Blueprints/Characters/BaseCharacter/BP_TacticalChar.BP_TacticalChar_C"))
      (set `self.PlayerCharacters` _outactors)
      (`self.CalculateTurn`))))

(event `self.ReceiveTick`
  (params (DeltaSeconds :type "Float (single-precision)"))
  (if (`|EnumEquality` (`self.CurrentState`) "NewEnumerator0")
    (if (not (`self.CameraOverride`))
      (`/Game/Blueprints/Core/BP_CameraPawn.ReceiveLocationRef` (`self.CameraPawn`) (`self.K2_GetActorLocation` (`self.ActiveCharacter`))))))

(event `OnActionSelected`
  (params (Action :type "/Game/Blueprints/Core/EActionState Enum" :default "NewEnumerator2"))
  (bind _output_get (set `self.ActionState` Action))
  (switch `/Game/Blueprints/Core/EActionState` _output_get
    (:`NewEnumerator0`
      (set `self.IsSelectingDestination` true)
      (`Widget.RemoveFromParent` (`self.ActionMenuInstance`)))))

(event `EnhancedInput|/Game/Input/Actions/IA_ToggleSpectatorMode`
  (params (ActionValue :type Boolean) (ElapsedSeconds :type "Float (double-precision)") (TriggeredSeconds :type "Float (double-precision)") (InputAction :type "InputAction Object Reference" :default "/Game/Input/Actions/IA_ToggleSpectatorMode.IA_ToggleSpectatorMode"))
  ; Menu controls
  (:`Triggered`
    (`self.CalculateTurn`)))

(event `EnhancedInput|/Game/Input/Actions/IA_ToggleMenu`
  (params (ActionValue :type Boolean) (ElapsedSeconds :type "Float (double-precision)") (TriggeredSeconds :type "Float (double-precision)") (InputAction :type "InputAction Object Reference" :default "/Game/Input/Actions/IA_ToggleMenu.IA_ToggleMenu"))
  ; Menu controls
  (:`Triggered`
    (if (`|EnumEquality` (`self.CurrentState`) "NewEnumerator2")
      (`self.SwitchToState` (`self.PreviousState`))
      (else
        (set `self.PreviousState` (`self.CurrentState`))
        (`self.SwitchToState` "NewEnumerator2")))))

(event `EnhancedInput|/Game/Input/Actions/IA_Cancel`
  (params (ActionValue :type Boolean) (ElapsedSeconds :type "Float (double-precision)") (TriggeredSeconds :type "Float (double-precision)") (InputAction :type "InputAction Object Reference" :default "/Game/Input/Actions/IA_Cancel.IA_Cancel"))
  (:`Triggered`
    (set `self.ActionState` "NewEnumerator2")
    (set `self.IsSelectingDestination` false)
    (`UserWidget.AddToViewport` (`self.ActionMenuInstance`) 0)))

(event `EnhancedInput|/Game/Input/Actions/IA_ZoomCamera`
  (params (ActionValue :type "Float (double-precision)") (ElapsedSeconds :type "Float (double-precision)") (TriggeredSeconds :type "Float (double-precision)") (InputAction :type "InputAction Object Reference" :default "/Game/Input/Actions/IA_ZoomCamera.IA_ZoomCamera"))
  ; Camera controls
  (:`Triggered`
    (`/Game/Blueprints/Core/BP_CameraPawn.ReceiveMoveInstruction` (`self.CameraPawn`) ActionValue (0.0 0.0) (0.0 0.0))))

(event `EnhancedInput|/Game/Input/Actions/IA_MoveCamera`
  (params (ActionValue :type "Vector2D Structure") (ElapsedSeconds :type "Float (double-precision)") (TriggeredSeconds :type "Float (double-precision)") (InputAction :type "InputAction Object Reference" :default "/Game/Input/Actions/IA_MoveCamera.IA_MoveCamera"))
  ; Camera controls
  (:`Triggered`
    (`/Game/Blueprints/Core/BP_CameraPawn.ReceiveMoveInstruction` (`self.CameraPawn`) 0.0 ActionValue (0.0 0.0))
    (set `self.CameraOverride` true)))

(event `EnhancedInput|/Game/Input/Actions/IA_LookCamera`
  (params (ActionValue :type "Vector2D Structure") (ElapsedSeconds :type "Float (double-precision)") (TriggeredSeconds :type "Float (double-precision)") (InputAction :type "InputAction Object Reference" :default "/Game/Input/Actions/IA_LookCamera.IA_LookCamera"))
  ; Camera controls
  (:`Triggered`
    (`/Game/Blueprints/Core/BP_CameraPawn.ReceiveMoveInstruction` (`self.CameraPawn`) 0.0 (0.0 0.0) ActionValue)))

(event `EnhancedInput|/Game/Input/Actions/IA_ClickSelect`
  (params (ActionValue :type Boolean) (ElapsedSeconds :type "Float (double-precision)") (TriggeredSeconds :type "Float (double-precision)") (InputAction :type "InputAction Object Reference" :default "/Game/Input/Actions/IA_ClickSelect.IA_ClickSelect"))
  (bind (_bblockinghit _binitialoverlap _time _distance _location) (`GameplayStatics.BreakHitResult` (`self.GetHitResultUnderCursorByChannel` "TraceTypeQuery1")))
  (:`Triggered`
    (if (`self.IsSelectingDestination`)
      (if _bblockinghit
        (message `/Game/Blueprints/Core/BPI_PlayerInstructions.RequestMove` (`self.ActiveCharacter`) (`self.AIController`) _location)
        (set `self.CameraOverride` false)
        (set `self.IsSelectingDestination` false)
        (set `self.ActionState` "NewEnumerator2")
        (`UserWidget.AddToViewport` (`self.ActionMenuInstance`) 0)))))

(fn `CalculateTurn`
  (locals (MaxTurnPoints :type "Float (double-precision)") (IsTurnTriggered :type Boolean))
  (bind _playercharacters (`self.PlayerCharacters`))
  (bind _activecharacter (`self.ActiveCharacter`))
  (if (> (`KismetArrayLibrary.Array_Length` _playercharacters) 0)
    (bind _output_get (set `local.IsTurnTriggered` true))
    (while _output_get
      (for _array_element _playercharacters
        (bind _speed (`/Game/Blueprints/Characters/BaseCharacter/BP_TacticalChar.Speed` _array_element))
        (bind _output_get_2 (set `/Game/Blueprints/Characters/BaseCharacter/BP_TacticalChar.TurnPoints` (+ (`KismetMathLibrary.RandomFloatInRange` (* _speed 0.8) _speed) (`/Game/Blueprints/Characters/BaseCharacter/BP_TacticalChar.TurnPoints` _array_element)) _array_element))
        (if (> _output_get_2 (`local.MaxTurnPoints`))
          (bind _output_get_3 (set `local.MaxTurnPoints` _output_get_2))
          (set `self.ActiveCharacter` _array_element)
          (`KismetSystemLibrary.PrintString` (`KismetStringLibrary.Conv_DoubleToString` _output_get_3))))
      (if (>= (`local.MaxTurnPoints`) (`self.TurnTrigger`))
        (set `/Game/Blueprints/Characters/BaseCharacter/BP_TacticalChar.TurnPoints` (- (`/Game/Blueprints/Characters/BaseCharacter/BP_TacticalChar.TurnPoints` _activecharacter) (`self.TurnTrigger`)) _activecharacter)
        (set `local.MaxTurnPoints` 0.0)
        (set `local.IsTurnTriggered` false)))
    (`KismetSystemLibrary.PrintString` "Turn triggered")
    (`self.StartNewTurn`)
    (`self.Possess` (`self.AIController`) (`self.ActiveCharacter`))
    (`self.SetViewTargetWithBlend` (`self.CameraPawn`))
    (`KismetSystemLibrary.PrintString` "has turn")
    (`KismetSystemLibrary.PrintString` (`KismetSystemLibrary.GetDisplayName` (`self.ActiveCharacter`)))))

(fn `SelectAction`
  (params (SelectedAction :type "/Game/Blueprints/Core/EActionState Enum" :default "NewEnumerator0"))
  (bind _output_get (set `self.ActionState` SelectedAction))
  (switch `/Game/Blueprints/Core/EActionState` _output_get
    (:`NewEnumerator0`
      (set `self.IsSelectingDestination` true))))

(fn `StartNewTurn`
  (`UserWidget.AddToViewport` (`self.ActionMenuInstance`) 0))

(fn `SwitchToState`
  (params (NewState :type "/Game/Blueprints/Core/EGameState Enum" :default "NewEnumerator0"))
  (bind _output (`|GetArrayItem` (`self.PlayerCharacters`)))
  (bind _output_get (set `self.CurrentState` NewState))
  (switch `/Game/Blueprints/Core/EGameState` _output_get
    (:`NewEnumerator0`
      (`self.Possess` _output)
      (set `self.ActiveCharacter` _output)
      (`Widget.RemoveFromParent` (`self.PauseMenuInstance`))
      (`self.SetViewTargetWithBlend` (`self.CameraPawn`)))
    (:`NewEnumerator1`
      (`self.Possess` (`self.CameraPawn`))
      (`Widget.RemoveFromParent` (`self.PauseMenuInstance`)))
    (:`NewEnumerator2`
      (`self.UnPossess`)
      (`UserWidget.AddToViewport` (`self.PauseMenuInstance`) 0))))

(fn `UserConstructionScript`)