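; BP_TBPawn is a camera pawn with smoothed zoom, movement and rotation.
; ReceiveMoveInstruction turns inputs into targets: clamped spring arm length, location along the actor's forward and right vectors, arm pitch and actor yaw.
; ReceiveLocationRef overrides the location target directly.
; Tick interpolates the spring arm and actor toward these targets, which BeginPlay seeds from their initial state.
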(event `self.ReceiveBeginPlay`
  (bind _springarm (`self.SpringArm`))
  (set `self.Zoom_Ref` (`SpringArmComponent.TargetArmLength` _springarm))
  (set `self.Location_Ref` (`self.K2_GetActorLocation`))
  (set `self.Rotation_Ref` (`self.K2_GetActorRotation`))
  (set `self.ArmRotation_Ref` (`SpringArmComponent.GetTargetRotation` _springarm)))

(event `self.ReceiveTick`
  (params (DeltaSeconds :type "Float (single-precision)"))
  (bind _springarm (`self.SpringArm`))
  (set `SpringArmComponent.TargetArmLength` (`KismetMathLibrary.FInterpTo` (`SpringArmComponent.TargetArmLength` _springarm) (`self.Zoom_Ref`) DeltaSeconds (`self.Zoom_Interp`)) _springarm)
  (`SceneComponent.K2_SetRelativeRotation` (`self.SpringArm`) (`KismetMathLibrary.RInterpTo` (`SceneComponent.RelativeRotation` (`self.SpringArm`)) (`self.ArmRotation_Ref`) DeltaSeconds (`self.Rotation_Interp`)) false false)
  (`self.K2_SetActorLocation` (`KismetMathLibrary.VInterpTo` (`self.K2_GetActorLocation`) (`self.Location_Ref`) DeltaSeconds (`self.Move_Interp`)))
  (`self.K2_SetActorRotation` (`KismetMathLibrary.RInterpTo` (`self.K2_GetActorRotation`) (`self.Rotation_Ref`) DeltaSeconds (`self.Rotation_Interp`))))

(fn `ReceiveLocationRef`
  (params (NewLocation :type "Vector Structure"))
  (set `self.Location_Ref` NewLocation))

(fn `ReceiveMoveInstruction`
  (params (ZoomInput :type "Float (double-precision)") (MoveInput :type "Vector2D Structure") (RotationInput :type "Vector2D Structure"))
  (bind (_x _y) (`KismetMathLibrary.BreakVector2D` MoveInput))
  (bind (_x_2 _y_2) (`KismetMathLibrary.BreakVector2D` RotationInput))
  ; Set zoom
  (set `self.Zoom_Ref` (`KismetMathLibrary.FClamp` (+ (`self.Zoom_Ref`) (* ZoomInput (`self.Zoom_Speed`))) (`self.Zoom_Min`) (`self.Zoom_Max`)))
  ; Set location
  (set `self.Location_Ref` (+ (`self.Location_Ref`) (* (* _x (`self.Move_Speed`)) (`self.GetActorForwardVector`))))
  (set `self.Location_Ref` (+ (`self.Location_Ref`) (* (* _y (`self.Move_Speed`)) (`self.GetActorRightVector`))))
  ; Set rotation
  (set `self.ArmRotation_Ref` (`KismetMathLibrary.ComposeRotators` (`self.ArmRotation_Ref`) (`KismetMathLibrary.MakeRotator` 0.0 (* _x_2 (`self.Rotation_Speed`)))))
  (set `self.Rotation_Ref` (`KismetMathLibrary.ComposeRotators` (`self.Rotation_Ref`) (`KismetMathLibrary.MakeRotator` 0.0 0.0 (* _y_2 (`self.Rotation_Speed`))))))

(fn `UserConstructionScript`)